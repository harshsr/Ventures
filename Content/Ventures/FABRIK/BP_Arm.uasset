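; BP_Arm is an arm actor that drives a poseable mesh with a FABRIK inverse kinematics chain component.
; The construction script assigns PoseableMesh as the chain of FabrikChainComp.
; On BeginPlay and every Tick, it passes the world transforms of Target and Pole to the component as its single target and pole target.
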(event `self.ReceiveBeginPlay`
  (bind _fabrikchaincomp (`self.FabrikChainComp`))
  (set `FabrikChainComp.TargetTransforms` (`|MakeArray` (`SceneComponent.K2_GetComponentToWorld` (`self.Target`))) _fabrikchaincomp)
  (set `FabrikChainComp.PoleTargets` (`|MakeArray` (`SceneComponent.K2_GetComponentToWorld` (`self.Pole`))) _fabrikchaincomp))

(event `self.ReceiveTick`
  (params (DeltaSeconds :type "Float (single-precision)"))
  (bind _fabrikchaincomp (`self.FabrikChainComp`))
  (set `FabrikChainComp.TargetTransforms` (`|MakeArray` (`SceneComponent.K2_GetComponentToWorld` (`self.Target`))) _fabrikchaincomp)
  (set `FabrikChainComp.PoleTargets` (`|MakeArray` (`SceneComponent.K2_GetComponentToWorld` (`self.Pole`))) _fabrikchaincomp))

(fn `UserConstructionScript`
  (set `FabrikChainComp.Chain` (`self.PoseableMesh`) (`self.FabrikChainComp`)))