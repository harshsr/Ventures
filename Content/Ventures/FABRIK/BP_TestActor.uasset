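; Test actor for a procedurally walking monster that moves forward on nine FABRIK IK chains.
; When a chain nears full extension, a sphere trace down from its pole picks a new ground target.
; Each tick eases chain targets toward those points and moves body height toward the targets' vertical midpoint plus its starting offset.
; A line trace through the body gradually tilts it to the ground normal.
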(event `self.ReceiveBeginPlay`
  (bind (_returnvalue_x _returnvalue_y _returnvalue_z) (`KismetMathLibrary.BreakVector` (`SceneComponent.K2_GetComponentLocation` (`self.InitialOffset`))))
  (bind (_returnvalue_x_2 _returnvalue_y_2 _returnvalue_z_2) (`KismetMathLibrary.BreakVector` (`SceneComponent.K2_GetComponentLocation` (`self.Monster`))))
  (for (_array_element _array_index) (`self.TargetsArr`)
    (`KismetArrayLibrary.Array_Set` (`self.TargetLocations`) _array_index (`SceneComponent.K2_GetComponentToWorld` _array_element)))
  (set `FabrikChainComp.TargetTransforms` (`self.TargetLocations`) (`self.FabrikChainComp`))
  (set `self.InitialZOffset` (- _returnvalue_z_2 _returnvalue_z)))

(event `self.ReceiveTick`
  (params (DeltaSeconds :type "Float (single-precision)"))
  (`SceneComponent.K2_AddWorldOffset` (`self.Monster`) (* (`self.GetActorForwardVector`) (* DeltaSeconds (`self.Speed`))) false false)
  (`self.SetIKData`)
  (`self.VerticalOffset`)
  (`self.Alignment`))

(fn `Alignment`
  (locals (LocationsArray :type "Array of Vector Structure"))
  (bind _monster (`self.Monster`))
  (bind _monster_2 (`self.Monster`))
  (bind _monster_3 (`self.Monster`))
  (bind _returnvalue (`SceneComponent.K2_GetComponentLocation` _monster))
  (bind _returnvalue_2 (`SceneComponent.GetUpVector` _monster))
  (bind _outhit (`KismetSystemLibrary.LineTraceSingle` :`Start` (+ _returnvalue (* _returnvalue_2 500.0)) :`End` (+ _returnvalue (* _returnvalue_2 -1000.0)) :`TraceChannel` "TraceTypeQuery3" :`DrawDebugType` "ForOneFrame"))
  (`SceneComponent.K2_SetWorldRotation` _monster_3 (`KismetMathLibrary.RInterpTo` (`SceneComponent.K2_GetComponentRotation` _monster_3) (`KismetMathLibrary.MakeRotationFromAxes` (`SceneComponent.GetForwardVector` _monster_2) (`SceneComponent.GetRightVector` _monster_2) (`.Normal` (`GameplayStatics.BreakHitResult` _outhit))) (`GameplayStatics.GetWorldDeltaSeconds`) 1.0) false false))

(fn `RecalculateTarget`
  (params (Index :type Integer))
  (locals (ChainInd :type Integer) (Radius1 :type "Float (double-precision)" :default 150.0) (Radius2 :type "Float (double-precision)" :default 10.0) (Radius3 :type "Float (double-precision)" :default 15.0))
  (`|ExecutionSequence`
    (:`then_0`
      (bind _output_get (set `local.ChainInd` Index))
      (bind _output (`|GetArrayItem` (`self.PolesArr`) _output_get))
      (bind _returnvalue (`SceneComponent.K2_GetComponentLocation` _output))
      (bind _outhit (`KismetSystemLibrary.SphereTraceSingle` _returnvalue (+ _returnvalue (* (`SceneComponent.GetUpVector` _output) -500.0)) (`local.Radius1`) "TraceTypeQuery3"))
      (if (`GameplayStatics.BreakHitResult` _outhit)
        (`KismetArrayLibrary.Array_Set` (`self.TargetLocations`) (`local.ChainInd`) (`KismetMathLibrary.MakeTransform` (`.ImpactPoint` (`GameplayStatics.BreakHitResult` _outhit)) (`SceneComponent.K2_GetComponentRotation` (`|GetArrayItem` (`self.TargetsArr`) (`local.ChainInd`)))))))))

(fn `SetIKData`
  (bind _fabrikchaincomp (`self.FabrikChainComp`))
  (`|ExecutionSequence`
    (:`then_0`
      (for _index (range 9)
        (bind _returnvalue (`FabrikChainComp.GetExtensionRatio` (`self.FabrikChainComp`) _index))
        (if (> _returnvalue 0.95)
          (`self.RecalculateTarget` _index))))
    (:`then_1`
      (for (_array_element _array_index) (`self.TargetLocations`)
        (bind _returnvalue_2 (`FabrikChainComp.GetTargetTransformByChainIndex` _fabrikchaincomp _array_index))
        (`FabrikChainComp.SetTargetTransformByChainIndex` _fabrikchaincomp _array_index (`KismetMathLibrary.MakeTransform` (`KismetMathLibrary.VInterpTo` (.location _returnvalue_2) (.location _array_element) (`GameplayStatics.GetWorldDeltaSeconds`) 10.0) (.rotation _array_element) (.scale _array_element)))))))

(fn `UserConstructionScript`
  (bind _polesarr (`self.PolesArr`))
  (bind _targetsarr (`self.TargetsArr`))
  (set `FabrikChainComp.Chain` (`self.Monster`) (`self.FabrikChainComp`))
  (`|ExecutionSequence`
    (:`then_0`
      (`KismetArrayLibrary.Array_Add` _targetsarr (`self.Target_C`))
      (`KismetArrayLibrary.Array_Add` _targetsarr (`self.Target_F`))
      (`KismetArrayLibrary.Array_Add` _targetsarr (`self.Target_R`))
      (`KismetArrayLibrary.Array_Add` _targetsarr (`self.Target_Lft`))
      (`KismetArrayLibrary.Array_Add` _targetsarr (`self.Target_Rgt`))
      (`KismetArrayLibrary.Array_Add` _targetsarr (`self.Target_FL`))
      (`KismetArrayLibrary.Array_Add` _targetsarr (`self.Target_FR`))
      (`KismetArrayLibrary.Array_Add` _targetsarr (`self.Target_RL`))
      (`KismetArrayLibrary.Array_Add` _targetsarr (`self.Target_RR`)))
    (:`then_1`
      (`KismetArrayLibrary.Array_Add` _polesarr (`self.Pole_C`))
      (`KismetArrayLibrary.Array_Add` _polesarr (`self.Pole_F`))
      (`KismetArrayLibrary.Array_Add` _polesarr (`self.Pole_R`))
      (`KismetArrayLibrary.Array_Add` _polesarr (`self.Pole_Lft`))
      (`KismetArrayLibrary.Array_Add` _polesarr (`self.Pole_Rght`))
      (`KismetArrayLibrary.Array_Add` _polesarr (`self.Pole_FL`))
      (`KismetArrayLibrary.Array_Add` _polesarr (`self.Pole_FR`))
      (`KismetArrayLibrary.Array_Add` _polesarr (`self.Pole_RL`))
      (`KismetArrayLibrary.Array_Add` _polesarr (`self.Pole_RR`)))))

(fn `VerticalOffset`
  (locals (SmallestZ :type "Float (double-precision)" :default 118753.504888) (BiggestZ :type "Float (double-precision)"))
  (bind _biggestz (`local.BiggestZ`))
  (bind _monster (`self.Monster`))
  (bind (_returnvalue_x _returnvalue_y _returnvalue_z) (`KismetMathLibrary.BreakVector` (`SceneComponent.K2_GetComponentLocation` _monster)))
  (`|ExecutionSequence`
    (:`then_0`
      (for _array_element (`self.TargetLocations`)
        (if (< (.z (.location _array_element)) (`local.SmallestZ`))
          (set `local.SmallestZ` (.z (.location _array_element))))
        (if (> (.z (.location _array_element)) (`local.BiggestZ`))
          (set `local.BiggestZ` (.z (.location _array_element))))))
    (:`then_1`
      (set `self.DesiredVerticleZ` (+ (- _biggestz (/ (- _biggestz (`local.SmallestZ`)) 2.0)) (`self.InitialZOffset`)))
      (`SceneComponent.K2_SetWorldLocation` _monster (`KismetMathLibrary.MakeVector` _returnvalue_x _returnvalue_y (`KismetMathLibrary.FInterpTo_Constant` _returnvalue_z (`self.DesiredVerticleZ`) (`GameplayStatics.GetWorldDeltaSeconds`) 25.0)) false false))))